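; Voxel chunk Blueprint that computes a 2D simplex noise grid for its chunk, likely as terrain heights.
; CalculateNoise loops over the chunk's cells row by row, offsetting by chunk index so sampling continues across neighboring chunks.
; Scaled coordinates feed SimplexNoise2D, and each weighted, floored result is appended to the returned Noise array without clearing it first.
; The event graph and construction script are empty.
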(event EventBeginPlay)

(event Collision|EventActorBeginOverlap
  (params (OtherActor :type Actor%20Object%20Reference)))

(event EventTick
  (params (DeltaSeconds :type Float%20%28single-precision%29)))

(fn ConstructionScript)

(fn CalculateNoise
  (bind _chunklineelements (Variables|Default|GetchunkLineElements))
  (bind _noise (LocalVariables|Getnoise))
  (bind _returnvalue (- _chunklineelements 1))
  (for _index (range 0 _returnvalue)
    (LocalVariables|SetyLoc _index)
    (for _index_2 (range 0 _returnvalue)
      (LocalVariables|SetxLoc _index_2)
      (bind _returnvalue_2 (Class|SimplexNoiseBPLibrary|SimplexNoise2D (* (+ (LocalVariables|GetxLoc) (* (Variables|Default|GetchunkXIndex) (Variables|Default|GetchunkLineElements))) (Variables|Default|GetxMult)) (* (+ (LocalVariables|GetyLoc) (* (Variables|Default|GetchunkYIndex) (Variables|Default|GetchunkLineElements))) (Variables|Default|GetyMult)) 1.0))
      (Utilities|Array|Add _noise (Math|Float|Floor (* _returnvalue_2 (Variables|Default|Getweight))))))
  (return _noise))